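; Wall actor that the player rotates around its local yaw axis with the Left and Right keys.
; On BeginPlay it enables input and switches the first player's view to the second CameraActor returned by a level-wide search.
; Each Tick it polls both keys into a signed direction, then applies a local rotation scaled by RotationSpeed and delta time.
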(event EventBeginPlay
  (bind _returnvalue (Game|GetPlayerController 0))
  (Input|EnableInput _returnvalue)
  (bind _outactors (Actor|GetAllActorsOfClass "/Script/Engine.CameraActor"))
  (Game|Player|SetViewTargetwithBlend _returnvalue (Utilities|Array|Get(acopy) _outactors 1) 0.0 "VTBlend_Linear" 0.0 false))

(event EventTick
  (params (DeltaSeconds :type Float%20%28single-precision%29))
  (Variables|Default|Setdirection 0)
  (if (Game|Player|IsInputKeyDown (Game|GetPlayerController 0) "Right")
    (Variables|Default|Setdirection (+ (Variables|Default|Getdirection) 1)))
  (if (Game|Player|IsInputKeyDown (Game|GetPlayerController 0) "Left")
    (Variables|Default|Setdirection (+ (Variables|Default|Getdirection) -1)))
  (Transformation|AddActorLocalRotation (Math|Rotator|MakeRotator 0.0 0.0 (* DeltaSeconds (Variables|Default|GetrotationSpeed) (Math|Conversions|ToFloat(Integer) (Variables|Default|Getdirection)))) false false))

(fn ConstructionScript)