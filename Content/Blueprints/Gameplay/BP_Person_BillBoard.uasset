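; Billboard person actor that wanders randomly on the horizontal plane until hit by a wall pawn or it escapes.
; A looping two-second timer picks a new random direction and speed, and Tick eases between the previous and new directions.
; Beyond a fixed radius from the world origin it counts as escaped, sinks downward and calls Destroy after a delay.
; Wall overlap calls Destroy immediately, which only sets an AutoDestroyWhenFinished flag.
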(event OnComponentBeginOverlap(Capsule)
  (params (OverlappedComponent :type Primitive%20Component%20Object%20Reference) (OtherActor :type Actor%20Object%20Reference) (OtherComp :type Primitive%20Component%20Object%20Reference) (OtherBodyIndex :type Integer) (bFromSweep :type Boolean) (SweepResult :type Hit%20Result%20Structure%20%28by%20ref%29))
  (Utilities|Casting|CastToBP_Wall_Pawn OtherActor)
  (Development|PrintString "Hit by wall")
  (CallFunction|Destroy))

(event EventBeginPlay
  (CallFunction|GenerateMovement)
  (Utilities|Time|SetTimerbyFunctionName 0 "GenerateMovement" 2.0 true))

(event EventTick
  (params (DeltaSeconds :type Float%20%28single-precision%29))
  (bind _capsule (Variables|Default|GetCapsule))
  (bind _returnvalue (Transformation|GetWorldLocation _capsule))
  (if (Variables|Default|GetEscaped)
    (Transformation|SetActorLocation (+ (* "0, 0,-100.000000" DeltaSeconds) (Transformation|GetWorldLocation (Variables|Default|GetCapsule))) false false)
    (else
      (bind _output_get (Variables|Default|SetInterpAlpha (+ (* DeltaSeconds 0.25) (Variables|Default|GetInterpAlpha))))
      (Transformation|SetActorLocation (+ (* (* (Math|Vector|Normalize (Math|Vector|Lerp(Vector) (Variables|Default|GetPreviousDirection) (Variables|Default|GetMoveDirection) _output_get)) (Variables|Default|GetMoveSpeed)) DeltaSeconds) _returnvalue) false false)
      (Math|Float|CompareFloat (Math|Vector|VectorLength (- "0, 0, 0" _returnvalue)) 255.0
        (:>
          (Development|PrintString "Escaped")
          (Variables|Default|SetEscaped true)
          (Utilities|Time|SetTimerbyFunctionName 0 "Destroy" 5.0))))))

(fn ConstructionScript)

(fn GenerateMovement
  (Variables|Default|SetInterpAlpha 0.0)
  (Variables|Default|SetMoveSpeed (* (Variables|Default|GetBaseMoveSpeed) (Math|Random|RandomFloatinRange 1.0 1.5)))
  (Variables|Default|SetPreviousDirection (Variables|Default|GetMoveDirection))
  (bind _direction (CallFunction|GetRandomMovement))
  (Variables|Default|SetMoveDirection _direction))

(fn GetRandomMovement
  (return (Math|Vector|Normalize (Math|Vector|MakeVector (Math|Random|RandomFloatinRange -1.0 1.0) (Math|Random|RandomFloatinRange -1.0 1.0) 0.0))))

(fn Destroy
  (Variables|Default|SetbAutoDestroyWhenFinished true))