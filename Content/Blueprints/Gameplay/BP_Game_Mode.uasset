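; Game mode that spawns a BP_Wall_Pawn at the world origin for each player who logs in and possesses it.
; It also adapts difficulty through KillEnemy and MissEnemy events, which keep running totals and streak-independent counters.
; Every 15 kills raises DifficultyLevel, gated by MaxLevel, and every 5 misses lowers it, down to zero.
; A check on 16 total misses exists but both branches are empty.
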(event Custom|Event%20KillEnemy
  (bind _difficultylevel (Variables|Default|GetDifficultyLevel))
  (Math|Integer|IncrementInt (Variables|Default|GetEnemiesKilledTotal)
    (:%20%20
      (bind _result (Math|Integer|IncrementInt (Variables|Default|GetEnemiesKilled))
        (:%20%20
          (if (> _result 14)
            (Variables|Default|SetEnemiesKilled 0)
            (if (<= _difficultylevel (Variables|Default|GetMaxLevel))
              (Math|Integer|IncrementInt _difficultylevel))))))))

(event Custom|Event%20MissEnemy
  (bind _difficultylevel (Variables|Default|GetDifficultyLevel))
  (bind _result (Math|Integer|IncrementInt (Variables|Default|GetEnemiesMissedTotal))
    (:%20%20
      (if (>= _result 16)
        _
        (else
          _))
      (bind _result_2 (Math|Integer|IncrementInt (Variables|Default|GetEnemiesMissed))
        (:%20%20
          (if (> _result_2 4)
            (Variables|Default|SetEnemiesMissed 0)
            (if (> _difficultylevel 0)
              (Math|Integer|DecrementInt _difficultylevel))))))))

(event EventBeginPlay)

(event EventTick
  (params (DeltaSeconds :type Float%20%28single-precision%29)))

(event EventPostLogin
  (params (NewPlayer :type Player%20Controller%20Object%20Reference))
  (bind _returnvalue (Game|SpawnActorfromClass "/Game/Blueprints/Gameplay/BP_Wall_Pawn.BP_Wall_Pawn_C" (Math|Transform|MakeTransform "0, 0, 0") "Undefined" 0 0))
  (Pawn|Possess NewPlayer _returnvalue))

(fn ConstructionScript)