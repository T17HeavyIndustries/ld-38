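; Enemy actor that dies when it overlaps the wall pawn, notifying the game mode of a kill, or of a miss through FuncMissed.
; Construction randomly makes a small share of enemies tin-hat variants, shown by a different billboard material, that survive one hit.
; That hit reverses the movement direction, derives a randomly angled PreviousDirection from it and restores the normal walk material.
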(event OnComponentBeginOverlap(Capsule)
  (params (OverlappedComponent :type Primitive%20Component%20Object%20Reference) (OtherActor :type Actor%20Object%20Reference) (OtherComp :type Primitive%20Component%20Object%20Reference) (OtherBodyIndex :type Integer) (bFromSweep :type Boolean) (SweepResult :type Hit%20Result%20Structure%20%28by%20ref%29))
  (bind _capsule (Variables|Default|GetCapsule))
  (Utilities|Casting|CastToBP_Wall_Pawn OtherActor)
  (if (== (Variables|Default|GetBounces) 0)
    (Rendering|SetVisibility _capsule false false)
    (Collision|SetCollisionEnabled _capsule "NoCollision")
    (Default|EventKillEnemy (Variables|Default|GetGameModeRef))
    (CallFunction|Destroy)
    (else
      (bind _output_get (Variables|Default|SetBounces (- (Variables|Default|GetBounces) 1)))
      (bind _output_get_2 (Variables|Default|SetMoveDirection (* (+ (Variables|Default|GetMoveDirection) (Variables|Default|GetPreviousDirection)) -1.0)))
      (Variables|Default|SetPreviousDirection (Math|Vector|RotateVectorAroundAxis _output_get_2 (Math|Random|RandomFloatinRange -45.0 45.0) "0, 0,1.000000"))
      (if (== _output_get 0)
        (Rendering|Material|SetMaterial (Variables|Default|GetMaterialBillboard) 0 "/Game/Materials/Mat_Walk_Anim.Mat_Walk_Anim")))))

(event EventBeginPlay
  (|CallParentFunction))

(event EventTick
  (params (DeltaSeconds :type Float%20%28single-precision%29))
  (|CallParentFunction DeltaSeconds))

(event EventFuncMissed
  (Default|EventMissEnemy (Variables|Default|GetGameModeRef))
  (|CallParentFunction))

(fn ConstructionScript
  (|CallParentFunction)
  (bind _output_get (Variables|Default|SetBounces (Math|Integer|SelectInt 0 1 (Math|Random|RandomBoolwithWeight 0.9))))
  (if (not (== _output_get 0))
    (Rendering|Material|SetMaterial (Variables|Default|GetMaterialBillboard) 0 "/Game/Materials/Mat_TinHat_Walk_Anim.Mat_TinHat_Walk_Anim")))