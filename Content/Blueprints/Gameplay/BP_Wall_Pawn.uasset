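; Player pawn that spins a wall via Positive and Negative input, while the spring arm camera rotates on its own.
; Tick rotates EarthWallWall1 by the summed input direction and the spring arm by a separate camera direction.
; Wall size and rotation speed events step through four clamped levels, toggling mesh visibility and collision or picking a speed.
; Each change also randomizes the camera's spin direction.
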(event Custom|Event%20WallIncrease
  (bind _output_get (Variables|PowerUps|SetWallSize (Math|Integer|Clamp(Integer) (+ (Variables|PowerUps|GetWallSize) 1) 0 3)))
  (CallFunction|FuncSetWallSize (Utilities|Array|Get(acopy) (Variables|PowerUps|GetWalls) _output_get))
  (CallFunction|FuncChangeCameraRotation))

(event Custom|Event%20WallDecrease
  (bind _output_get (Variables|PowerUps|SetWallSize (Math|Integer|Clamp(Integer) (+ (Variables|PowerUps|GetWallSize) -1) 0 3)))
  (CallFunction|FuncSetWallSize (Utilities|Array|Get(acopy) (Variables|PowerUps|GetWalls) _output_get))
  (CallFunction|FuncChangeCameraRotation))

(event Custom|Event%20SpeedIncrease
  (bind _output_get (Variables|PowerUps|SetSpeed_Level (Math|Integer|Clamp(Integer) (+ (Variables|PowerUps|GetSpeed_Level) 1) 0 3)))
  (Variables|Movement|SetRotationSpeed (Utilities|Array|Get(acopy) (Variables|PowerUps|GetSpeeds) _output_get))
  (CallFunction|FuncChangeCameraRotation))

(event Custom|Event%20SpeedDecrease
  (bind _output_get (Variables|PowerUps|SetSpeed_Level (Math|Integer|Clamp(Integer) (+ (Variables|PowerUps|GetSpeed_Level) -1) 0 3)))
  (Variables|Movement|SetRotationSpeed (Utilities|Array|Get(acopy) (Variables|PowerUps|GetSpeeds) _output_get))
  (CallFunction|FuncChangeCameraRotation))

(event EventBeginPlay
  (Input|EnableInput (Game|GetPlayerController 0)))

(event EventDestroyed)

(event EventTick
  (params (DeltaSeconds :type Float%20%28single-precision%29))
  (Utilities|FlowControl|Sequence
    (:then_0
      (Transformation|AddLocalRotation (Variables|Default|GetEarthWall_Wall_1) (Math|Rotator|MakeRotator 0.0 0.0 (* DeltaSeconds (Variables|Default|GetrotationSpeed) (Math|Conversions|ToFloat(Integer) (Variables|Default|Getdirection)))) false false))
    (:then_1
      (Transformation|AddWorldRotation (Variables|Default|GetSpringArm) (Math|Rotator|MakeRotator 0.0 0.0 (* DeltaSeconds (Variables|Movement|GetCameraRotationSpeed) (Math|Conversions|ToFloat(Integer) (Variables|Movement|GetCameraDirection)))) false false))))

(event EventPossessed
  (params (NewController :type Controller%20Object%20Reference)))

(event EventUnpossessed
  (params (OldController :type Controller%20Object%20Reference)))

(event Input|ActionEvents|InputActionPositive
  (params (Key :type Key%20Structure :default "AnyKey"))
  (:Pressed
    (if (not (Variables|Movement|GetPositiveDown))
      (Variables|Movement|SetPositiveDown true)
      (Variables|Default|Setdirection (+ (Variables|Default|Getdirection) 1))))
  (:Released
    (if (Variables|Movement|GetPositiveDown)
      (Variables|Movement|SetPositiveDown false)
      (Variables|Movement|SetDirection (+ (Variables|Default|Getdirection) -1)))))

(event Input|ActionEvents|InputActionNegative
  (params (Key :type Key%20Structure :default "AnyKey"))
  (:Pressed
    (if (not (Variables|Movement|GetNegativeDown))
      (Variables|Movement|SetNegativeDown true)
      (Variables|Default|Setdirection (+ (Variables|Default|Getdirection) -1))))
  (:Released
    (if (Variables|Movement|GetNegativeDown)
      (Variables|Movement|SetNegativeDown false)
      (Variables|Movement|SetDirection (+ (Variables|Default|Getdirection) 1)))))

(fn ConstructionScript
  (bind _earthwall_wall_2 (Variables|Default|GetEarthWall_Wall_2))
  (Utilities|FlowControl|Sequence
    (:then_0
      (bind _output_get (Variables|PowerUps|SetWalls (Utilities|Array|MakeArray (Variables|Default|GetEarthWall_Wall_1) (Variables|Default|GetEarthWall_Wall_2) (Variables|Default|GetEarthWall_Wall_3) (Variables|Default|GetEarthWall_Wall_4))))
      (for _array_element _output_get
        (Rendering|SetVisibility _array_element false false)
        (Collision|SetCollisionEnabled _array_element "NoCollision"))
      (Rendering|SetVisibility _earthwall_wall_2 true false)
      (Collision|SetCollisionEnabled _earthwall_wall_2 "QueryAndPhysics")
      (Variables|PowerUps|SetWallSize 1))
    (:then_1
      (Variables|PowerUps|SetSpeeds (Utilities|Array|MakeArray (Variables|PowerUps|GetSpeed1) (Variables|PowerUps|GetSpeed2) (Variables|PowerUps|GetSpeed3) (Variables|PowerUps|GetSpeed4)))
      (Variables|PowerUps|SetSpeed_Level 1))))

(fn FuncSetWallSize
  (params (Wall :type Static%20Mesh%20Component%20Object%20Reference))
  (for _array_element (Variables|PowerUps|GetWalls)
    (if (!= _array_element Wall)
      (Rendering|SetVisibility _array_element false false)
      (Collision|SetCollisionEnabled _array_element "NoCollision")))
  (Rendering|SetVisibility Wall true false)
  (Collision|SetCollisionEnabled Wall "QueryAndPhysics"))

(fn FuncChangeCameraRotation
  (if (Math|Random|RandomBool)
    (Variables|Movement|SetCameraDirection 1)
    (else
      (Variables|Movement|SetCameraDirection -1))))