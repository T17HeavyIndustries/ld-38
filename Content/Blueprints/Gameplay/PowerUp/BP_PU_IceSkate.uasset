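; BP_PU_IceSkate is an ice skate power-up pickup that speeds up the wall pawn that touches it.
; When its capsule overlaps a BP_Wall_Pawn, it plays a pickup sound at the world origin, then hides the capsule and disables its collision.
; It then calls the pawn's EventSpeedIncrease, which handles the boost itself, and destroys itself.
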(event OnComponentBeginOverlap(Capsule)
  (params (OverlappedComponent :type Primitive%20Component%20Object%20Reference) (OtherActor :type Actor%20Object%20Reference) (OtherComp :type Primitive%20Component%20Object%20Reference) (OtherBodyIndex :type Integer) (bFromSweep :type Boolean) (SweepResult :type Hit%20Result%20Structure%20%28by%20ref%29))
  (bind _capsule (Variables|Default|GetCapsule))
  (bind _asbp_wall_pawn (Utilities|Casting|CastToBP_Wall_Pawn OtherActor))
  (Audio|SpawnSoundatLocation "/Game/sounds/PU_4_Cue.PU_4_Cue" "0, 0, 0")
  (Rendering|SetVisibility _capsule false false)
  (Collision|SetCollisionEnabled _capsule "NoCollision")
  (Default|EventSpeedIncrease _asbp_wall_pawn)
  (CallFunction|Destroy))

(event EventBeginPlay
  (|CallParentFunction))

(event Collision|EventActorBeginOverlap
  (params (OtherActor :type Actor%20Object%20Reference)))

(event EventTick
  (params (DeltaSeconds :type Float%20%28single-precision%29))
  (|CallParentFunction DeltaSeconds))

(fn ConstructionScript
  (|CallParentFunction))