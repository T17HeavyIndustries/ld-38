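; Wandering beaker power-up that triggers a wall increase when BP_Wall_Pawn touches it.
; A looping timer randomizes speed and turns the heading, which Tick blends for smooth horizontal drift.
; Nearing the edge of a radius around world origin freezes heading changes; crossing it makes the beaker sink.
; Pickup hides the capsule and calls Destroy, also timed after escape, which only sets AutoDestroyWhenFinished.
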(event OnComponentBeginOverlap(Capsule)
  (params (OverlappedComponent :type Primitive%20Component%20Object%20Reference) (OtherActor :type Actor%20Object%20Reference) (OtherComp :type Primitive%20Component%20Object%20Reference) (OtherBodyIndex :type Integer) (bFromSweep :type Boolean) (SweepResult :type Hit%20Result%20Structure%20%28by%20ref%29))
  (bind _capsule (Variables|Default|GetCapsule))
  (bind _asbp_wall_pawn (Utilities|Casting|CastToBP_Wall_Pawn OtherActor))
  (Development|PrintString "Hit by wall")
  (Rendering|SetVisibility _capsule false false)
  (Collision|SetCollisionEnabled _capsule "NoCollision")
  (Default|EventWallIncrease _asbp_wall_pawn)
  (CallFunction|Destroy))

(event EventBeginPlay
  (CallFunction|GenerateMovement)
  (Utilities|Time|SetTimerbyFunctionName 0 "GenerateMovement" 2.0 true))

(event EventTick
  (params (DeltaSeconds :type Float%20%28single-precision%29))
  (bind _capsule (Variables|Default|GetCapsule))
  (bind _returnvalue (Transformation|GetWorldLocation _capsule))
  (bind _returnvalue_2 (- "0, 0, 0" _returnvalue))
  (bind _returnvalue_3 (Math|Vector|VectorLength _returnvalue_2))
  (if (Variables|Default|GetEscaped)
    (Transformation|SetActorLocation (+ (* "0, 0,-100.000000" DeltaSeconds) (Transformation|GetWorldLocation (Variables|Default|GetCapsule))) false false)
    (else
      (bind _output_get (Variables|Default|SetInterpAlpha (+ (* DeltaSeconds 0.25) (Variables|Default|GetInterpAlpha))))
      (Transformation|SetActorLocation (+ (* (* (Math|Vector|Normalize (Math|Vector|Lerp(Vector) (Variables|Default|GetPreviousDirection) (Variables|Default|GetMoveDirection) _output_get)) (Variables|Default|GetMoveSpeed)) DeltaSeconds) _returnvalue) false false)
      (if (>= _returnvalue_3 2.3e+02)
        (Variables|Default|SetStopNewMovement true))
      (Math|Float|CompareFloat _returnvalue_3 255.0
        (:>
          (Development|PrintString "Escaped")
          (Variables|Default|SetEscaped true)
          (Utilities|Time|SetTimerbyFunctionName 0 "Destroy" 5.0))))))

(fn ConstructionScript)

(fn GenerateMovement
  (if (Variables|Default|GetStopNewMovement)
    (Development|PrintString "Stop")
    (else
      (if (Variables|Default|GetInitial)
        (Variables|Default|SetInitial false)
        (bind _direction (CallFunction|GetRandomMovement))
        (Variables|Default|SetMoveDirection _direction))
      (Variables|Default|SetInterpAlpha 0.0)
      (Variables|Default|SetMoveSpeed (* (Variables|Default|GetBaseMoveSpeed) (Math|Random|RandomFloatinRange 1.0 1.5)))
      (Variables|Default|SetPreviousDirection (Variables|Default|GetMoveDirection))
      (Variables|Default|SetMoveDirection (Math|Vector|RotateVectorAroundAxis (Variables|Default|GetMoveDirection) (Math|Random|RandomFloatinRange -9e+01 9e+01) "0, 0,1.000000")))))

(fn GetRandomMovement
  (return (Math|Vector|Normalize (Math|Vector|MakeVector (Math|Random|RandomFloatinRange -1.0 1.0) (Math|Random|RandomFloatinRange -1.0 1.0) 0.0))))

(fn Destroy
  (Variables|Default|SetbAutoDestroyWhenFinished true))