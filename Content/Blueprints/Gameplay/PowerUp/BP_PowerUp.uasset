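; Power-up actor that drifts around the world origin in random horizontal directions until it escapes.
; A looping timer rerolls speed and heading, and Tick blends from the previous direction to the new one for curved motion.
; Past set distances from origin it stops rerolling, then sinks and starts a missed timer calling Destroy, which only sets AutoDestroyWhenFinished.
; Capsule overlap is empty; the wall-hit logic calling EventWallDecrease is disconnected.
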(event OnComponentBeginOverlap(Capsule)
  (params (OverlappedComponent :type Primitive%20Component%20Object%20Reference) (OtherActor :type Actor%20Object%20Reference) (OtherComp :type Primitive%20Component%20Object%20Reference) (OtherBodyIndex :type Integer) (bFromSweep :type Boolean) (SweepResult :type Hit%20Result%20Structure%20%28by%20ref%29)))

(event EventBeginPlay
  (bind _asbp_game_mode (Utilities|Casting|CastToBP_Game_Mode (Game|GetGameMode)))
  (Variables|Default|SetGameModeRef _asbp_game_mode)
  (CallFunction|GenerateMovement)
  (Utilities|Time|SetTimerbyFunctionName 0 "GenerateMovement" 2.0 true))

(event EventTick
  (params (DeltaSeconds :type Float%20%28single-precision%29))
  (bind _capsule (Variables|Default|GetCapsule))
  (bind _returnvalue (Transformation|GetWorldLocation _capsule))
  (bind _returnvalue_2 (- "0, 0, 0" _returnvalue))
  (bind _returnvalue_3 (Math|Vector|VectorLength _returnvalue_2))
  (if (Variables|Default|GetEscaped)
    (Transformation|SetActorLocation (+ (* "0, 0,-100.000000" DeltaSeconds) (Transformation|GetWorldLocation (Variables|Default|GetCapsule))) false false))
  (bind _output_get (Variables|Default|SetInterpAlpha (+ (* DeltaSeconds 0.25) (Variables|Default|GetInterpAlpha))))
  (Transformation|SetActorLocation (+ (* (* (Math|Vector|Normalize (Math|Vector|Lerp(Vector) (Variables|Default|GetPreviousDirection) (Variables|Default|GetMoveDirection) _output_get)) (Variables|Default|GetMoveSpeed)) DeltaSeconds) _returnvalue) false false)
  (if (>= _returnvalue_3 2.3e+02)
    (Variables|Default|SetStopNewMovement true))
  (if (> _returnvalue_3 255.0)
    (if (not (Variables|Default|GetEscaped))
      (Variables|Default|SetEscaped true)
      (Utilities|Time|SetTimerbyFunctionName 0 "FuncMissed" 4.0))))

(fn ConstructionScript)

(fn GenerateMovement
  (if (not (Variables|Default|GetStopNewMovement))
    (if (Variables|Default|GetInitial)
      (Variables|Default|SetInitial false)
      (bind _direction (CallFunction|GetRandomMovement))
      (Variables|Default|SetMoveDirection _direction))
    (Variables|Default|SetInterpAlpha 0.0)
    (Variables|Default|SetMoveSpeed (* (Variables|Default|GetBaseMoveSpeed) (Math|Random|RandomFloatinRange 1.0 1.5)))
    (Variables|Default|SetPreviousDirection (Variables|Default|GetMoveDirection))
    (Variables|Default|SetMoveDirection (Math|Vector|RotateVectorAroundAxis (Variables|Default|GetMoveDirection) (Math|Random|RandomFloatinRange -9e+01 9e+01) "0, 0,1.000000"))))

(fn GetRandomMovement
  (return (Math|Vector|Normalize (Math|Vector|MakeVector (Math|Random|RandomFloatinRange -1.0 1.0) (Math|Random|RandomFloatinRange -1.0 1.0) 0.0))))

(fn Destroy
  (Variables|Default|SetbAutoDestroyWhenFinished true))

(fn FuncMissed
  (CallFunction|Destroy))