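; BP_PowerUp_Manager periodically spawns random power-up pickups into the level.
; The construction script fills the PowerUps array with the beaker and fire billboard classes.
; BeginPlay starts a looping two-second timer that calls SpawnPerson, which despite its name spawns a random class from that array.
; Spawn positions are random X/Y points in a small square around the world origin at fixed height, independent of the manager's own location.
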(event EventBeginPlay
  (Utilities|Time|SetTimerbyFunctionName 0 "SpawnPerson" 2.0 true))

(fn ConstructionScript
  (Variables|Default|SetPowerUps (Utilities|Array|MakeArray "/Game/Blueprints/Gameplay/PowerUp/BP_Beaker_BillBoard.BP_Beaker_BillBoard_C" "/Game/Blueprints/Gameplay/PowerUp/BP_Fire_BillBoard.BP_Fire_BillBoard_C")))

(fn SpawnPerson
  (bind _powerups (Variables|Default|GetPowerUps))
  (Game|SpawnActorfromClass (Utilities|Array|Get(acopy) _powerups (Math|Random|RandomIntegerinRange 0 (- (Utilities|Array|Length _powerups) 1))) (Math|Transform|MakeTransform (Math|Vector|MakeVector (Math|Random|RandomFloatinRange -5e+01 5e+01) (Math|Random|RandomFloatinRange -5e+01 5e+01) 4e+01)) "Undefined" 0 0))