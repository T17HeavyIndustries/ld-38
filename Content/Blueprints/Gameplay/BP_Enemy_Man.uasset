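; BP_Enemy_Man is an enemy spawn manager that repeatedly spawns BP_Enemy at a random spot near the world origin.
; After an initial delay, its spawn event loops on a randomized retriggerable delay that shortens as the game mode's DifficultyLevel rises.
; Despite the PowerUp naming, the selection function always returns BP_Enemy; a weighted branch to BP_PU_TinHat is left disconnected.
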(event Custom|Event%20SpawnPowerUp
  (bind _gamemoderef (Variables|Default|GetGameModeRef))
  (bind _leveldifference (Variables|Default|GetLevelDifference))
  (bind _spawnmax (Variables|Default|GetSpawnMax))
  (bind _difficultylevel (Variables|/Game/Blueprints/Gameplay/BP_Game_Mode.BP_Game_Mode_C|GetDifficultyLevel _gamemoderef))
  (bind _returnvalue (* _difficultylevel _leveldifference))
  (bind _returnvalue_2 (- _spawnmax _returnvalue))
  (bind _powerup (CallFunction|FuncSelectPowerUp))
  (Game|SpawnActorfromClass _powerup (Math|Transform|MakeTransform (Math|Vector|MakeVector (Math|Random|RandomFloatinRange -5e+01 5e+01) (Math|Random|RandomFloatinRange -5e+01 5e+01) 4e+01)) "Undefined" 0 0)
  (Utilities|FlowControl|RetriggerableDelay (Math|Random|RandomFloatinRange (- _returnvalue_2 (Variables|Default|GetSpawnRange)) _returnvalue_2))
  (CallFunction|EventSpawnPowerUp))

(event EventBeginPlay
  (bind _asbp_game_mode (Utilities|Casting|CastToBP_Game_Mode (Game|GetGameMode)))
  (Variables|Default|SetGameModeRef _asbp_game_mode)
  (Utilities|FlowControl|Delay (Variables|Default|GetSpawnMax))
  (CallFunction|EventSpawnPowerUp))

(fn ConstructionScript)

(fn FuncSelectPowerUp
  (return "/Game/Blueprints/Gameplay/BP_Enemy.BP_Enemy_C"))